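; BP_ZE is an actor that rotates a Cube from readings sent by an Arduino over a serial connection.
; On BeginPlay it opens a COM port, prints whether that succeeded and, if so, starts a fast looping timer that polls the port for a string.
; Each successful read is printed and converted to a number that sets both roll and pitch of the Cube's world rotation, with yaw held at zero.
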(event `self.ReceiveBeginPlay`
  (bind (_bopened _returnvalue) (`SerialCom.OpenComPort` 3))
  (if _bopened
    (`KismetSystemLibrary.PrintString` "Hello")
    (set `self.Arduino` _returnvalue)
    (`KismetSystemLibrary.K2_SetTimerDelegate` (delegate `Loop`) 0.1 true)
    (else
      (`KismetSystemLibrary.PrintString` "Nao"))))

(event `Loop`
  (bind (_bsuccess _returnvalue) (`SerialCom.ReadString` (`self.Arduino`)))
  (if _bsuccess
    (`KismetSystemLibrary.PrintString` _returnvalue)
    (bind _returnvalue_2 (`KismetStringLibrary.Conv_StringToDouble` _returnvalue))
    (`SceneComponent.K2_SetWorldRotation` (`self.Cube`) (`KismetMathLibrary.MakeRotator` _returnvalue_2 _returnvalue_2) true false)))

(fn `UserConstructionScript`)